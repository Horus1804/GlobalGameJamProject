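; BP_GunPlayer is a short-lived gun actor that hands the player's gun to BP_KroopaToopa on contact.
; On spawn it spins its mesh via a timeline, then after a short delay re-shows the player's mesh and destroys itself.
; Overlapping KroopaToopa transfers the gun, starts its fire, costs player life, increments score, updates the HUD and respawns the player at zero life.
; Any overlap destroys the actor.
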(event OnComponentBeginOverlap(Box)
  (params (OverlappedComponent :type Primitive%20Component%20Object%20Reference) (OtherActor :type Actor%20Object%20Reference) (OtherComp :type Primitive%20Component%20Object%20Reference) (OtherBodyIndex :type Integer) (bFromSweep :type Boolean) (SweepResult :type Hit%20Result%20Structure%20%28by%20ref%29))
  (bind _kroopatoopa_ref (Variables|Default|GetKroopaToopa%20ref))
  (bind _player_ref (Variables|Default|GetPlayer%20ref))
  (bind _hud_ref (Variables|/Game/ThirdPerson/Blueprints/BP_ThirdPersonCharacter.BP_ThirdPersonCharacter_C|GetHUD%20ref _player_ref))
  ;[1 1 1] Hit element
  (Development|PrintString "Hello")
  (if (== OtherActor (Variables|Default|GetKroopaToopa%20ref))
    (Variables|/Game/Guillaume/BPs/Enemies/KroopaToopa/BP_KroopaToopa.BP_KroopaToopa_C|SetHave%20gun _kroopatoopa_ref true)
    (Default|VisibilityGun _kroopatoopa_ref)
    (Default|StartFire _kroopatoopa_ref)
    (Variables|/Game/ThirdPerson/Blueprints/BP_ThirdPersonCharacter.BP_ThirdPersonCharacter_C|SetHave%20gun _player_ref false)
    (Default|VisibilityGun _player_ref)
    (Variables|/Game/ThirdPerson/Blueprints/BP_ThirdPersonCharacter.BP_ThirdPersonCharacter_C|SetLife _player_ref (- (Variables|/Game/ThirdPerson/Blueprints/BP_ThirdPersonCharacter.BP_ThirdPersonCharacter_C|GetLife _player_ref) 1e+01))
    (Default|SetLife _hud_ref)
    (Default|Painfull _hud_ref)
    (Variables|/Game/ThirdPerson/Blueprints/BP_ThirdPersonCharacter.BP_ThirdPersonCharacter_C|SetScore _player_ref (+ (Variables|/Game/ThirdPerson/Blueprints/BP_ThirdPersonCharacter.BP_ThirdPersonCharacter_C|GetScore _player_ref) 1))
    (Default|CoinsScore (Variables|/Game/ThirdPerson/Blueprints/BP_ThirdPersonCharacter.BP_ThirdPersonCharacter_C|GetHUD%20ref _player_ref))
    (if (<= (Variables|/Game/ThirdPerson/Blueprints/BP_ThirdPersonCharacter.BP_ThirdPersonCharacter_C|GetLife _player_ref) 0.0)
      (Default|Respawn _player_ref))
    (Actor|DestroyActor)
    (else
      (Actor|DestroyActor))))

(event Custom|rotatemesh
  ;[1 1 1] rotate
  (bind _newtrack_0 (Timeline|Timeline Play)
    (:Update
      (Transformation|SetWorldRotation (Variables|Default|GetStaticMesh) (Math|Rotator|MakeRotator (.x _newtrack_0) 0.0 0.0) false false))))

(event EventBeginPlay
  ;[1 1 1] Begin play
  (bind _asbp_third_person_character (Utilities|Casting|CastToBP_ThirdPersonCharacter (Game|GetPlayerCharacter 0)))
  (Variables|Default|SetPlayer%20ref _asbp_third_person_character)
  (bind _returnvalue (Actor|GetActorOfClass "/Game/Guillaume/BPs/Enemies/KroopaToopa/BP_KroopaToopa.BP_KroopaToopa_C"))
  (Variables|Default|SetKroopaToopa%20ref _returnvalue)
  (bind _returnvalue_2 (Actor|GetActorOfClass "/Game/Mathis/Blueprint/BP_Pickup.BP_Pickup_C"))
  (Variables|Default|SetPickup%20ref _returnvalue_2)
  (CallFunction|Rotatemesh)
  (Utilities|FlowControl|Delay 1.0)
  (Rendering|SetVisibility (Variables|/Game/ThirdPerson/Blueprints/BP_ThirdPersonCharacter.BP_ThirdPersonCharacter_C|GetStaticMesh (Variables|Default|GetPlayer%20ref)) true false)
  (Actor|DestroyActor))

(fn ConstructionScript)