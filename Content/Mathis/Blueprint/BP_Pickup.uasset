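; Collectible pickup actor whose Pickup enum selects its mesh at BeginPlay and its effect on the player.
; A timeline rotates the mesh; box overlap applies the effect: coins lower score, potatoes raise it, others change movement or grant gun or dictionary.
; Effect names run counter-intuitive: the speed ring sets slow movement, iron boots fast.
; Pickup plays VFX and sound, then hides without being destroyed, so respawnobject can restore it.
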(event OnComponentBeginOverlap(Box)
  (params (OverlappedComponent :type Primitive%20Component%20Object%20Reference) (OtherActor :type Actor%20Object%20Reference) (OtherComp :type Primitive%20Component%20Object%20Reference) (OtherBodyIndex :type Integer) (bFromSweep :type Boolean) (SweepResult :type Hit%20Result%20Structure%20%28by%20ref%29))
  (bind _player_ref (Variables|Default|GetPlayer%20ref))
  (bind _player_ref_2 (Variables|Default|GetPlayer%20ref))
  (bind _player_ref_3 (Variables|Default|GetPlayer%20ref))
  (bind _charactermovement (Variables|/Script/Engine.Character|GetCharacterMovement _player_ref))
  ;[1 1 1] Coins add
  (if (== OtherActor _player_ref)
    (Niagara|SpawnSystematLocation "/Game/Guillaume/BPs/FX/ItemGot/NS_ItemGot.NS_ItemGot" (Transformation|GetWorldLocation (Variables|Default|GetBox)))
    (switch Utilities|FlowControl|Switch|SwitchonE_Pickup (Variables|Default|GetPickup)
      (:NewEnumerator0
        ;;[1 0.249 0.8003] Score
        (Variables|/Game/ThirdPerson/Blueprints/BP_ThirdPersonCharacter.BP_ThirdPersonCharacter_C|SetScore _player_ref (+ (Variables|/Game/ThirdPerson/Blueprints/BP_ThirdPersonCharacter.BP_ThirdPersonCharacter_C|GetScore _player_ref) -1))
        (Default|CoinsScore (Variables|/Game/ThirdPerson/Blueprints/BP_ThirdPersonCharacter.BP_ThirdPersonCharacter_C|GetHUD%20ref (Variables|Default|GetPlayer%20ref)) :!label _label))
      (:NewEnumerator1
        (Variables|/Game/ThirdPerson/Blueprints/BP_ThirdPersonCharacter.BP_ThirdPersonCharacter_C|SetScore _player_ref (+ (Variables|/Game/ThirdPerson/Blueprints/BP_ThirdPersonCharacter.BP_ThirdPersonCharacter_C|GetScore _player_ref) 1))
        (goto _label))
      (:NewEnumerator2
        ;;[0.4145 1 0.3402] Speed
        (Variables|/Script/Engine.CharacterMovementComponent|SetMaxAcceleration _charactermovement 2e+01)
        (Variables|/Script/Engine.CharacterMovementComponent|SetMaxWalkSpeed _charactermovement 2e+02)
        (Variables|/Game/ThirdPerson/Blueprints/BP_ThirdPersonCharacter.BP_ThirdPersonCharacter_C|SetBotte%20de%20fer%20take _player_ref_2 false))
      (:NewEnumerator3
        (Variables|/Script/Engine.CharacterMovementComponent|SetMaxAcceleration _charactermovement 4e+03)
        (Variables|/Script/Engine.CharacterMovementComponent|SetMaxWalkSpeed _charactermovement 2.5e+03)
        (Variables|/Game/ThirdPerson/Blueprints/BP_ThirdPersonCharacter.BP_ThirdPersonCharacter_C|SetBotte%20de%20fer%20take _player_ref_2 true))
      (:NewEnumerator4
        (bind _output_get (Variables|/Game/ThirdPerson/Blueprints/BP_ThirdPersonCharacter.BP_ThirdPersonCharacter_C|SetHave%20gun _player_ref_3 true))
        (Rendering|SetVisibility (Variables|/Game/ThirdPerson/Blueprints/BP_ThirdPersonCharacter.BP_ThirdPersonCharacter_C|GetStaticMesh _player_ref_3) _output_get false))
      (:NewEnumerator5
        (Variables|/Game/ThirdPerson/Blueprints/BP_ThirdPersonCharacter.BP_ThirdPersonCharacter_C|SetDictionnary _player_ref true)))
    (Collision|SetCollisionEnabled (Variables|Default|GetBox) "NoCollision")
    (Rendering|SetVisibility (Variables|Default|GetStaticMesh) false false)
    (Audio|SpawnSound2D "/Game/SFX/PickUpItem/Item_Pick_Up_SFX_Cue.Item_Pick_Up_SFX_Cue" 1.0 1.0 0.0 0)))

(event Custom|respawn%20object
  (bind _staticmesh (Variables|Default|GetStaticMesh))
  ;[1 1 1] Respawn
  (Rendering|SetVisibility _staticmesh true false)
  (Collision|SetCollisionEnabled _staticmesh "QueryAndPhysics")
  (Collision|SetCollisionEnabled (Variables|Default|GetBox) "QueryOnly"))

(event Custom|rotatemesh
  ;[1 1 1] rotate
  (bind _newtrack_0 (Timeline|Rotate Play)
    (:Update
      (Transformation|SetWorldRotation (Variables|Default|GetStaticMesh) (Math|Rotator|MakeRotator 0.0 0.0 (.z _newtrack_0)) false false))))

(event EventBeginPlay
  (bind _staticmesh (Variables|Default|GetStaticMesh))
  ;[1 1 1] begin play
  (bind _asbp_third_person_character (Utilities|Casting|CastToBP_ThirdPersonCharacter (Game|GetPlayerCharacter 0)))
  (Variables|Default|SetPlayer%20ref _asbp_third_person_character)
  (switch Utilities|FlowControl|Switch|SwitchonE_Pickup (Variables|Default|GetPickup)
    (:NewEnumerator0
      (Components|StaticMesh|SetStaticMesh _staticmesh "/Game/Assets/Coin_Low.Coin_Low"))
    (:NewEnumerator1
      (Components|StaticMesh|SetStaticMesh _staticmesh "/Game/Assets/Patate_Low.Patate_Low"))
    (:NewEnumerator2
      (Components|StaticMesh|SetStaticMesh _staticmesh "/Game/Assets/Bracelet_Low.Bracelet_Low"))
    (:NewEnumerator3
      (Components|StaticMesh|SetStaticMesh _staticmesh "/Game/Assets/Boots_Low.Boots_Low"))
    (:NewEnumerator4
      (Components|StaticMesh|SetStaticMesh _staticmesh "/Game/Assets/Gun_Low.Gun_Low"))
    (:NewEnumerator5
      (Components|StaticMesh|SetStaticMesh _staticmesh "/Game/LevelPrototyping/Meshes/SM_ChamferCube.SM_ChamferCube")))
  (CallFunction|Rotatemesh))

(fn ConstructionScript)