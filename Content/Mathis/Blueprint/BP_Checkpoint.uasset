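; BP_Checkpoint is a checkpoint actor that records the player's respawn point and score.
; On BeginPlay it casts player character 0 to BP_ThirdPersonCharacter and caches the reference.
; When that character overlaps the Box, it sets the character's RespawnLocation to the checkpoint's location with a fixed world X offset and copies Score into ScoreCheck.
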(event OnComponentBeginOverlap(Box)
  (params (OverlappedComponent :type Primitive%20Component%20Object%20Reference) (OtherActor :type Actor%20Object%20Reference) (OtherComp :type Primitive%20Component%20Object%20Reference) (OtherBodyIndex :type Integer) (bFromSweep :type Boolean) (SweepResult :type Hit%20Result%20Structure%20%28by%20ref%29))
  (bind _player_ref (Variables|Default|GetPlayer%20ref))
  (if (== OtherActor _player_ref)
    (Variables|/Game/ThirdPerson/Blueprints/BP_ThirdPersonCharacter.BP_ThirdPersonCharacter_C|SetRespawn%20location _player_ref (+ (Transformation|GetActorLocation) "100.000000,0.000000,0.000000"))
    (Variables|/Game/ThirdPerson/Blueprints/BP_ThirdPersonCharacter.BP_ThirdPersonCharacter_C|SetScore%20check _player_ref (Variables|/Game/ThirdPerson/Blueprints/BP_ThirdPersonCharacter.BP_ThirdPersonCharacter_C|GetScore _player_ref))))

(event EventBeginPlay
  ;[1 1 1] Begin play
  (bind _asbp_third_person_character (Utilities|Casting|CastToBP_ThirdPersonCharacter (Game|GetPlayerCharacter 0)))
  (Variables|Default|SetPlayer%20ref _asbp_third_person_character))

(fn ConstructionScript)