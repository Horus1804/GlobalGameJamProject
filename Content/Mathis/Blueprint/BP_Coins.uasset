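; BP_Coins is a pickup actor that changes the player's score when something overlaps its box, then destroys itself.
; At BeginPlay it caches the BP_ThirdPersonCharacter player and uses the Coins boolean to pick its mesh.
; When Coins is true it is a chamfer cube that subtracts a point, otherwise a cylinder that adds one.
; Overlap updates the cached player's Score and HUD without checking which actor entered.
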(event OnComponentBeginOverlap(Box)
  (params (OverlappedComponent :type Primitive%20Component%20Object%20Reference) (OtherActor :type Actor%20Object%20Reference) (OtherComp :type Primitive%20Component%20Object%20Reference) (OtherBodyIndex :type Integer) (bFromSweep :type Boolean) (SweepResult :type Hit%20Result%20Structure%20%28by%20ref%29))
  ;[1 1 1] Coins add
  (bind _player_ref (Variables|Default|GetPlayer%20ref)
    (:then
      (if (Variables|Default|GetCoins?)
        (Variables|/Game/ThirdPerson/Blueprints/BP_ThirdPersonCharacter.BP_ThirdPersonCharacter_C|SetScore _player_ref (+ (Variables|/Game/ThirdPerson/Blueprints/BP_ThirdPersonCharacter.BP_ThirdPersonCharacter_C|GetScore _player_ref) -1))
        (else
          (Variables|/Game/ThirdPerson/Blueprints/BP_ThirdPersonCharacter.BP_ThirdPersonCharacter_C|SetScore _player_ref (+ (Variables|/Game/ThirdPerson/Blueprints/BP_ThirdPersonCharacter.BP_ThirdPersonCharacter_C|GetScore _player_ref) 1))))
      (Default|CoinsScore (Variables|/Game/ThirdPerson/Blueprints/BP_ThirdPersonCharacter.BP_ThirdPersonCharacter_C|GetHUD%20ref (Variables|Default|GetPlayer%20ref)))
      (Actor|DestroyActor))
    (:else)))

(event EventBeginPlay
  (bind _staticmesh (Variables|Default|GetStaticMesh))
  ;[1 1 1] begin play
  (bind _asbp_third_person_character (Utilities|Casting|CastToBP_ThirdPersonCharacter (Game|GetPlayerCharacter 0)))
  (Variables|Default|SetPlayer%20ref _asbp_third_person_character)
  (if (Variables|Default|GetCoins?)
    (Components|StaticMesh|SetStaticMesh _staticmesh "/Game/LevelPrototyping/Meshes/SM_ChamferCube.SM_ChamferCube")
    (else
      (Components|StaticMesh|SetStaticMesh _staticmesh "/Game/LevelPrototyping/Meshes/SM_Cylinder.SM_Cylinder"))))

(fn ConstructionScript)