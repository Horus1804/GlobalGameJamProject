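; Keypad-locked door that shows a code-entry widget and mouse cursor when its trigger box is overlapped.
; The widget is created hidden at BeginPlay, revealed on overlap and hidden again when the overlap ends.
; The check event, not called within this Blueprint, disables door collision, plays the opening sequence and hides the UI.
; Hiding also resets the open flags and the widget's GoodCode, but leaves the cursor visible.
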(event OnComponentBeginOverlap(Box)
  (params (OverlappedComponent :type Primitive%20Component%20Object%20Reference) (OtherActor :type Actor%20Object%20Reference) (OtherComp :type Primitive%20Component%20Object%20Reference) (OtherBodyIndex :type Integer) (bFromSweep :type Boolean) (SweepResult :type Hit%20Result%20Structure%20%28by%20ref%29))
  (bind _ui_keypad_door_ref (Variables|Default|GetUI_Keypad_Door_Ref))
  (Variables|Default|GetPlayer_Ref
    (:then
      (Variables|/Script/Engine.PlayerController|SetbShowMouseCursor (Game|GetPlayerController 0) true)
      (Widget|SetVisibility _ui_keypad_door_ref "Visible")
      (Widget|SetRenderOpacity _ui_keypad_door_ref 1.0))
    (:else)))

(event OnComponentEndOverlap(Box)
  (params (OverlappedComponent :type Primitive%20Component%20Object%20Reference) (OtherActor :type Actor%20Object%20Reference) (OtherComp :type Primitive%20Component%20Object%20Reference) (OtherBodyIndex :type Integer))
  (Variables|Default|GetPlayer_Ref
    (:then
      (CallFunction|HideDoorUI))
    (:else)))

(event Custom|check
  (Variables|Default|SetOpen_Door true)
  (Collision|SetCollisionEnabled (Variables|Default|GetDoor) "NoCollision")
  (Class|ActorSequenceComponent|PlaySequence (Variables|Default|GetActorSequence))
  (bind _output_get (Variables|Default|SetHide_UI_Keypad_Door true))
  (if _output_get
    (CallFunction|HideDoorUI)))

(event Custom|Hide_Door_UI
  (bind _ui_keypad_door_ref (Variables|Default|GetUI_Keypad_Door_Ref))
  ;[1 1 1] Hide UI
  (Widget|SetVisibility _ui_keypad_door_ref "Hidden")
  (Widget|SetRenderOpacity _ui_keypad_door_ref 0.0)
  (Variables|Default|SetOpen_Door false)
  (Variables|Default|SetHide_UI_Keypad_Door false)
  (Variables|/Game/Julien/WBP_Keypad_Door.WBP_Keypad_Door_C|SetGood_Code (Variables|Default|GetUI_Keypad_Door_Ref) false)
  (Utilities|FlowControl|Delay 5.0))

(event EventBeginPlay
  ;[1 1 1] Begin play
  (Variables|Default|SetPlayer_Ref (.AsBP%20Third%20Person%20Character (Utilities|Casting|CastToBP_ThirdPersonCharacter (Game|GetPlayerCharacter 0))))
  (Variables|Default|SetOpen_Door false)
  (Variables|Default|SetHide_UI_Keypad_Door false)
  (bind _returnvalue (UserInterface|CreateWidget "/Game/Julien/WBP_Keypad_Door.WBP_Keypad_Door_C"))
  (bind _output_get (Variables|Default|SetUI_Keypad_Door_Ref _returnvalue))
  (UserInterface|Viewport|AddtoViewport _output_get 0)
  (Widget|SetVisibility (Variables|Default|GetUI_Keypad_Door_Ref) "Hidden")
  (Widget|SetRenderOpacity (Variables|Default|GetUI_Keypad_Door_Ref) 0.0))

(fn ConstructionScript)