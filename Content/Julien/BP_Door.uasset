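; BP_Door is a door actor that opens when the player is near it along the Y axis and the character's Lock flag is true.
; A looping timer from BeginPlay polls this condition instead of checking on Tick.
; On success, a DoOnce disables door collision, plays an ActorSequence for the opening and clears the timer.
; Tick only prints the door's world location for debugging.
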(event Custom|Open_Door_Event
  (Variables|Default|SetDoor_Position (.y (Transformation|GetWorldLocation (Variables|Default|GetDoor self))))
  (Variables|Default|SetPlayer_Position (.y (Transformation|GetWorldLocation (Variables|/Script/Engine.Character|GetCapsuleComponent (Variables|Default|GetPlayer_Ref)))))
  (if (and (Math|Float|NearlyEqual(Float) (Variables|Default|GetDoor_Position) (Variables|Default|GetPlayer_Position) 2e+02) (Variables|/Game/ThirdPerson/Blueprints/BP_ThirdPersonCharacter.BP_ThirdPersonCharacter_C|GetLock%20? (Variables|Default|GetPlayer_Ref)))
    (Utilities|FlowControl|DoOnce false
      (:Completed
        (Variables|Default|SetOpen_Door false)
        (Collision|SetCollisionEnabled (Variables|Default|GetDoor) "NoCollision")
        (Class|ActorSequenceComponent|PlaySequence (Variables|Default|GetActorSequence))
        (Utilities|Time|ClearandInvalidateTimerbyHandle (Variables|Default|GetOpen_Door_Event_Ref))))))

(event EventBeginPlay
  (Variables|Default|SetPlayer_Ref (.AsBP%20Third%20Person%20Character (Utilities|Casting|CastToBP_ThirdPersonCharacter (Game|GetPlayerCharacter 0))))
  (Variables|Default|SetOpen_Door false)
  (bind _returnvalue (Utilities|Time|SetTimerbyEvent (EventDispatchers|CreateEvent :!event Custom|Open_Door_Event) 1.2 true))
  (Variables|Default|SetOpen_Door_Event_Ref _returnvalue))

(event EventTick
  (params (DeltaSeconds :type Float%20%28single-precision%29))
  (Development|PrintString (Utilities|String|ToString(Vector) (Transformation|GetWorldLocation (Variables|Default|GetDoor self))) true true "(R=1.000000,G=0.000000,B=0.101598,A=1.000000)" 0.1))

(fn ConstructionScript)