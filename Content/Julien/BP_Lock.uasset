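; BP_Lock is a lock pickup that the third-person character collects by walking into it.
; On overlap with the box, it sets the character's Lock flag and starts a short one-shot timer, apparently bound to the pickup event.
; That event plays a pickup sound, hides the lock, disables the box collision and clears the timer; the actor is hidden rather than destroyed.
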(event OnComponentBeginOverlap(Lock_Box)
  (params (OverlappedComponent :type Primitive%20Component%20Object%20Reference) (OtherActor :type Actor%20Object%20Reference) (OtherComp :type Primitive%20Component%20Object%20Reference) (OtherBodyIndex :type Integer) (bFromSweep :type Boolean) (SweepResult :type Hit%20Result%20Structure%20%28by%20ref%29))
  ;[0.009985 0 1] Event Begin Overlap : Set player variable and launch "Event Pick_Up_Lock"
  (bind _asbp_third_person_character (Utilities|Casting|CastToBP_ThirdPersonCharacter OtherActor))
  (bind _output_get (Variables|Default|SetPlayer_Ref _asbp_third_person_character))
  (Variables|/Game/ThirdPerson/Blueprints/BP_ThirdPersonCharacter.BP_ThirdPersonCharacter_C|SetLock%20? _output_get true)
  (bind _returnvalue (Utilities|Time|SetTimerbyEvent (EventDispatchers|CreateEvent :!event Custom|Pïck_Up_Lock) 0.1))
  (Variables|Default|SetPick_Up_Lock_Event_Ref _returnvalue))

(event Custom|Pïck_Up_Lock
  ;[1 0 0] Event_Pick_Up_Lock
  (Audio|PlaySound2D "/Game/SFX/PickUpItem/Item_Pick_Up_SFX_Cue.Item_Pick_Up_SFX_Cue" 1.0 1.0 0.0 0 0)
  (Rendering|SetVisibility (Variables|Default|GetLock) false false)
  (Collision|SetCollisionEnabled (Variables|Default|GetLock_Box) "NoCollision")
  (Utilities|Time|ClearandInvalidateTimerbyHandle (Variables|Default|GetPick_Up_Lock_Event_Ref)))

(fn ConstructionScript)