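; BP_TalkingFriendo is a friendly talker actor that plays a multi-page dialogue with the player.
; Its box overlap caches the third-person character, then sets or clears that character's talker reference and Friend flag on entering and leaving.
; StartDiscussion creates a dialog widget, reverting its font if the player's Dictionnary flag is set.
; Continuediscussion advances through the text array, then removes the widget and clears the player's speaking state.
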(event OnComponentBeginOverlap(Box)
  (params (OverlappedComponent :type Primitive%20Component%20Object%20Reference) (OtherActor :type Actor%20Object%20Reference) (OtherComp :type Primitive%20Component%20Object%20Reference) (OtherBodyIndex :type Integer) (bFromSweep :type Boolean) (SweepResult :type Hit%20Result%20Structure%20%28by%20ref%29))
  (bind _asbp_third_person_character (Utilities|Casting|CastToBP_ThirdPersonCharacter OtherActor))
  (bind _as_bp_third_person_character (Variables|Default|GetAs%20BP%20Third%20Person%20Character)
    (:then
      _)
    (:else
      (Utilities|FlowControl|DoOnce false
        (:Completed
          (bind _output_get (Variables|Default|SetAs%20BP%20Third%20Person%20Character _asbp_third_person_character))))))
  (Variables|/Game/ThirdPerson/Blueprints/BP_ThirdPersonCharacter.BP_ThirdPersonCharacter_C|SetTalkerRef _as_bp_third_person_character self)
  (Variables|/Game/ThirdPerson/Blueprints/BP_ThirdPersonCharacter.BP_ThirdPersonCharacter_C|SetFriend _output_get true))

(event OnComponentEndOverlap(Box)
  (params (OverlappedComponent :type Primitive%20Component%20Object%20Reference) (OtherActor :type Actor%20Object%20Reference) (OtherComp :type Primitive%20Component%20Object%20Reference) (OtherBodyIndex :type Integer))
  (Utilities|Casting|CastToBP_ThirdPersonCharacter OtherActor)
  (bind _as_bp_third_person_character (Variables|Default|GetAs%20BP%20Third%20Person%20Character)
    (:then
      (Variables|/Game/ThirdPerson/Blueprints/BP_ThirdPersonCharacter.BP_ThirdPersonCharacter_C|SetFriend _as_bp_third_person_character false)
      (Variables|/Game/ThirdPerson/Blueprints/BP_ThirdPersonCharacter.BP_ThirdPersonCharacter_C|SetTalkerRef _as_bp_third_person_character 0))
    (:else)))

(event Custom|StartDiscussion
  ;[1 1 1] Begin Discussion
  (Variables|/Game/ThirdPerson/Blueprints/BP_ThirdPersonCharacter.BP_ThirdPersonCharacter_C|SetTrueSpeaking (Variables|Default|GetAs%20BP%20Third%20Person%20Character) true)
  (bind _returnvalue (UserInterface|CreateWidget "/Game/Guillaume/BPs/UI_Discussion/WBP_DialogBox.WBP_DialogBox_C"))
  (bind _output_get (Variables|Default|SetDialogue _returnvalue))
  (if (Variables|/Game/ThirdPerson/Blueprints/BP_ThirdPersonCharacter.BP_ThirdPersonCharacter_C|GetDictionnary (Variables|Default|GetAs%20BP%20Third%20Person%20Character))
    (Default|ChangeFontBack _output_get))
  (Default|SetText _output_get (Utilities|Array|Get(acopy) (Variables|Default|GetAllDialogueTexts)))
  (UserInterface|Viewport|AddtoViewport _output_get 0)
  (Variables|Default|SetPageNumber 1)
  (Variables|Default|SetStartedDiscussion true))

(event Custom|Continue%20discussion
  (bind _alldialoguetexts (Variables|Default|GetAllDialogueTexts))
  (bind _dialogue (Variables|Default|GetDialogue))
  (bind _pagenumber (Variables|Default|GetPageNumber))
  ;[1 1 1] Continue/End the Discussion
  (if (not (>= _pagenumber (Utilities|Array|Length _alldialoguetexts)))
    (Default|SetText _dialogue (Utilities|Array|Get(acopy) _alldialoguetexts _pagenumber))
    (Math|Integer|IncrementInt _pagenumber)
    (else
      (Widget|RemovefromParent _dialogue)
      (Variables|Default|SetStartedDiscussion false)
      (Variables|/Game/ThirdPerson/Blueprints/BP_ThirdPersonCharacter.BP_ThirdPersonCharacter_C|SetTrueSpeaking (Variables|Default|GetAs%20BP%20Third%20Person%20Character) false))))

(event EventBeginPlay)

(event Collision|EventActorBeginOverlap
  (params (OtherActor :type Actor%20Object%20Reference)))

(event EventTick
  (params (DeltaSeconds :type Float%20%28single-precision%29)))

(fn ConstructionScript)