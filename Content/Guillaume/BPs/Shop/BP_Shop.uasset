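; BP_Shop is a shop actor that lets the player open a buying interface while inside its trigger box.
; On BeginPlay it creates a dialog box and a shop UI widget, handing the latter a reference to itself.
; Box overlaps set or clear the third-person character's in-shop flag and shop reference, caching the player.
; BuyItem shows both widgets and the cursor; LeaveItems hides them and clears the player's TrueInShop flag.
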(event OnComponentBeginOverlap(Box)
  (params (OverlappedComponent :type Primitive%20Component%20Object%20Reference) (OtherActor :type Actor%20Object%20Reference) (OtherComp :type Primitive%20Component%20Object%20Reference) (OtherBodyIndex :type Integer) (bFromSweep :type Boolean) (SweepResult :type Hit%20Result%20Structure%20%28by%20ref%29))
  (bind _asbp_third_person_character (Utilities|Casting|CastToBP_ThirdPersonCharacter OtherActor))
  (Variables|Default|GetPlayerRef
    (:then
      _)
    (:else
      (Utilities|FlowControl|DoOnce false
        (:Completed
          (Variables|Default|SetPlayerRef _asbp_third_person_character)))))
  (Variables|/Game/ThirdPerson/Blueprints/BP_ThirdPersonCharacter.BP_ThirdPersonCharacter_C|SetIsInShop _asbp_third_person_character true)
  (Variables|/Game/ThirdPerson/Blueprints/BP_ThirdPersonCharacter.BP_ThirdPersonCharacter_C|SetshopRef _asbp_third_person_character self))

(event OnComponentEndOverlap(Box)
  (params (OverlappedComponent :type Primitive%20Component%20Object%20Reference) (OtherActor :type Actor%20Object%20Reference) (OtherComp :type Primitive%20Component%20Object%20Reference) (OtherBodyIndex :type Integer))
  (bind _asbp_third_person_character (Utilities|Casting|CastToBP_ThirdPersonCharacter OtherActor))
  (Variables|/Game/ThirdPerson/Blueprints/BP_ThirdPersonCharacter.BP_ThirdPersonCharacter_C|SetIsInShop _asbp_third_person_character false)
  (Variables|/Game/ThirdPerson/Blueprints/BP_ThirdPersonCharacter.BP_ThirdPersonCharacter_C|SetshopRef _asbp_third_person_character 0))

(event Custom|BuyItem
  (UserInterface|Viewport|AddtoViewport (Variables|Default|GetDialogBoxRef) 0)
  (Variables|/Script/Engine.PlayerController|SetbShowMouseCursor (Game|GetPlayerController 0) true))

(event Custom|LeaveItems
  (Widget|RemovefromParent (Variables|Default|GetDialogBoxRef))
  (Variables|/Script/Engine.PlayerController|SetbShowMouseCursor (Game|GetPlayerController 0) false)
  (Variables|/Game/ThirdPerson/Blueprints/BP_ThirdPersonCharacter.BP_ThirdPersonCharacter_C|SetTrueInShop (Variables|Default|GetPlayerRef) false))

(event EventBeginPlay
  (bind _returnvalue (UserInterface|CreateWidget "/Game/Guillaume/BPs/UI_Discussion/WBP_DialogBox.WBP_DialogBox_C"))
  (Variables|Default|SetDialogBoxRef _returnvalue)
  (bind _returnvalue_2 (UserInterface|CreateWidget "/Game/Guillaume/BPs/Shop/WBP_ShopUI.WBP_ShopUI_C"))
  (Variables|Default|SetShopUIRef _returnvalue_2)
  (Variables|/Game/Guillaume/BPs/Shop/WBP_ShopUI.WBP_ShopUI_C|SetShopRef _returnvalue_2 self))

(event Collision|EventActorBeginOverlap
  (params (OtherActor :type Actor%20Object%20Reference)))

(event EventTick
  (params (DeltaSeconds :type Float%20%28single-precision%29)))

(fn ConstructionScript)