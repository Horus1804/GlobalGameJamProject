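; BP_TutoTV is a tutorial display actor that shows a WBP_Tutorial widget when the player character is nearby.
; On BeginPlay it fills the widget with an action image, an input image sequence and tutorial text.
; Its Box overlap scales the widget up when BP_ThirdPersonCharacter enters and to zero when it leaves.
; A DoOnce on entry also switches the tutorial text to a Comic Sans font.
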(event OnComponentBeginOverlap(Box)
  (params (OverlappedComponent :type Primitive%20Component%20Object%20Reference) (OtherActor :type Actor%20Object%20Reference) (OtherComp :type Primitive%20Component%20Object%20Reference) (OtherBodyIndex :type Integer) (bFromSweep :type Boolean) (SweepResult :type Hit%20Result%20Structure%20%28by%20ref%29))
  (Utilities|Casting|CastToBP_ThirdPersonCharacter OtherActor)
  (Transformation|SetWorldScale3D (Variables|Default|GetWidget) "0.250000,0.250000,0.250000")
  (if true
    (Utilities|FlowControl|DoOnce false
      (:Completed
        (Class|TextBlock|SetFont (Variables|/Game/Guillaume/BPs/Tv/WBP_Tutorial.WBP_Tutorial_C|GetTutorialText1 (Variables|Default|GetAs%20WBP%20Tutorial)) (Utilities|Struct|MakeSlateFontInfo "/Engine/EngineFonts/ComicSansMS3_Font.ComicSansMS3_Font" 0 "(OutlineSize=0,bSeparateFillAlpha=False,bApplyOutlineToDropShadows=False,OutlineMaterial=None,OutlineColor=(R=0.000000,G=0.000000,B=0.000000,A=1.000000))" "None" 55.0 0 0.0))))))

(event OnComponentEndOverlap(Box)
  (params (OverlappedComponent :type Primitive%20Component%20Object%20Reference) (OtherActor :type Actor%20Object%20Reference) (OtherComp :type Primitive%20Component%20Object%20Reference) (OtherBodyIndex :type Integer))
  (Utilities|Casting|CastToBP_ThirdPersonCharacter OtherActor)
  (Transformation|SetWorldScale3D (Variables|Default|GetWidget) "0, 0, 0"))

(event EventBeginPlay
  (bind _aswbp_tutorial (Utilities|Casting|CastToWBP_Tutorial (UserInterface|GetWidget (Variables|Default|GetWidget))))
  (bind _output_get (Variables|Default|SetAs%20WBP%20Tutorial _aswbp_tutorial))
  (Default|SetupImage(Solo) _output_get true (Variables|Default|GetAction%20Image))
  (Default|SetupImage(Sequence) _output_get false (Variables|Default|GetInputs%20Images))
  (Default|SetText _output_get (Variables|Default|GetTutorial%20Text)))

(event Collision|EventActorBeginOverlap
  (params (OtherActor :type Actor%20Object%20Reference)))

(event EventTick
  (params (DeltaSeconds :type Float%20%28single-precision%29)))

(fn ConstructionScript)