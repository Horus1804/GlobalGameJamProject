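; BP_KroopaToopa is an enemy that affects the third-person player character while it overlaps the enemy's Box.
; A hit decrements Score, refreshes the HUD via CoinsScore and increases Life.
; CanHit gates hits and InRange tracks overlap until it ends.
; Only when Life reaches the threshold does it snap to MaxLife, then a delay re-enables hits and calls Check to repeat while in range.
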(event OnComponentBeginOverlap(Box)
  (params (OverlappedComponent :type Primitive%20Component%20Object%20Reference) (OtherActor :type Actor%20Object%20Reference) (OtherComp :type Primitive%20Component%20Object%20Reference) (OtherBodyIndex :type Integer) (bFromSweep :type Boolean) (SweepResult :type Hit%20Result%20Structure%20%28by%20ref%29))
  (bind _player_ref (Variables|Default|GetPlayer%20ref))
  ;[1 1 1] Hit player
  (if (Variables|Default|Getcan%20hit%20?)
    (if (== OtherActor _player_ref)
      (Variables|Default|Setcan%20hit%20? false)
      (Variables|Default|Setin%20range true)
      (Variables|/Game/ThirdPerson/Blueprints/BP_ThirdPersonCharacter.BP_ThirdPersonCharacter_C|SetScore _player_ref (+ (Variables|/Game/ThirdPerson/Blueprints/BP_ThirdPersonCharacter.BP_ThirdPersonCharacter_C|GetScore _player_ref) -1))
      (Default|CoinsScore (Variables|/Game/ThirdPerson/Blueprints/BP_ThirdPersonCharacter.BP_ThirdPersonCharacter_C|GetHUD%20ref _player_ref))
      (bind _output_get (Variables|/Game/ThirdPerson/Blueprints/BP_ThirdPersonCharacter.BP_ThirdPersonCharacter_C|SetLife _player_ref (+ (Variables|/Game/ThirdPerson/Blueprints/BP_ThirdPersonCharacter.BP_ThirdPersonCharacter_C|GetLife _player_ref) 1e+01)))
      (if (>= _output_get 1e+02)
        (Variables|/Game/ThirdPerson/Blueprints/BP_ThirdPersonCharacter.BP_ThirdPersonCharacter_C|SetLife _player_ref (Variables|/Game/ThirdPerson/Blueprints/BP_ThirdPersonCharacter.BP_ThirdPersonCharacter_C|GetMax%20life _player_ref))
        (Utilities|FlowControl|Delay 2.0)
        (Variables|Default|Setcan%20hit%20? true)
        (CallFunction|Check)))))

(event OnComponentEndOverlap(Box)
  (params (OverlappedComponent :type Primitive%20Component%20Object%20Reference) (OtherActor :type Actor%20Object%20Reference) (OtherComp :type Primitive%20Component%20Object%20Reference) (OtherBodyIndex :type Integer))
  ;[1 1 1] End check
  (if (== OtherActor (Variables|Default|GetPlayer%20ref))
    (Variables|Default|Setin%20range false)))

(event Custom|Check
  (bind _player_ref (Variables|Default|GetPlayer%20ref))
  ;[1 1 1] Hit player
  (if (Variables|Default|Getin%20range)
    (if (Variables|Default|Getcan%20hit%20?)
      (if (== (stale OnComponentBeginOverlap(Box) OtherActor) _player_ref)
        (Variables|Default|Setcan%20hit%20? false)
        (Variables|Default|Setin%20range true)
        (Variables|/Game/ThirdPerson/Blueprints/BP_ThirdPersonCharacter.BP_ThirdPersonCharacter_C|SetScore _player_ref (+ (Variables|/Game/ThirdPerson/Blueprints/BP_ThirdPersonCharacter.BP_ThirdPersonCharacter_C|GetScore _player_ref) -1))
        (Default|CoinsScore (Variables|/Game/ThirdPerson/Blueprints/BP_ThirdPersonCharacter.BP_ThirdPersonCharacter_C|GetHUD%20ref _player_ref))
        (bind _output_get (Variables|/Game/ThirdPerson/Blueprints/BP_ThirdPersonCharacter.BP_ThirdPersonCharacter_C|SetLife _player_ref (+ (Variables|/Game/ThirdPerson/Blueprints/BP_ThirdPersonCharacter.BP_ThirdPersonCharacter_C|GetLife _player_ref) 1e+01)))
        (if (>= _output_get 1e+02)
          (Variables|/Game/ThirdPerson/Blueprints/BP_ThirdPersonCharacter.BP_ThirdPersonCharacter_C|SetLife _player_ref (Variables|/Game/ThirdPerson/Blueprints/BP_ThirdPersonCharacter.BP_ThirdPersonCharacter_C|GetMax%20life _player_ref))
          (Utilities|FlowControl|Delay 2.0)
          (Variables|Default|Setcan%20hit%20? true)
          (CallFunction|Check))))))

(event EventBeginPlay
  ;[1 1 1] Begin play
  (bind _asbp_third_person_character (Utilities|Casting|CastToBP_ThirdPersonCharacter (Game|GetPlayerCharacter 0)))
  (Variables|Default|SetPlayer%20ref _asbp_third_person_character))

(fn ConstructionScript)